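; Spline-driven mesh actor that sways with wind, building one non-colliding spline mesh segment per span between spline points.
; The construction script creates, shapes and scales the segments from the spline.
; Tick nudges segment positions and tangents along WindDirection by time-based sine and cosine waves, scaled by WindMagnitude over Scale.
; A half-sine along spline length pins both ends; offsets accumulate each frame, making sway frame-rate dependent.
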(event EventBeginPlay
  (Variables|Default|SetSplineMesh_Backup (Variables|Default|GetSplineMesh)))

(event EventActorBeginOverlap
  (params (OtherActor :type Actor%20Object%20Reference)))

(event EventTick
  (params (DeltaSeconds :type Float%20%28single-precision%29))
  (bind _spline (Variables|Default|GetSpline))
  (bind _returnvalue (Spline|GetSplineLength _spline))
  (for _index (range 0 (- (Spline|GetNumberOfSplinePoints _spline) 1))
    (Utilities|IsValid (Utilities|Array|Get(acopy) (Variables|Default|GetSplineMesh) _index)
      (:Is%20Valid
        (SplineMesh|SetStartPosition (Utilities|Array|Get(acopy) (Variables|Default|GetSplineMesh) _index) (+ (* (* (Math|Vector|GetForwardVector (Variables|Default|GetWindDirection)) (* (Math|Trig|Sin(Radians) (Variables|Default|Gett)) (/ (Variables|Default|GetWindMagnitude) (Variables|Default|GetScale)))) (Math|Trig|Sin(Radians) (Math|Float|MultiplybyPi (/ (Spline|GetDistanceAlongSplineatSplinePoint _spline _index) _returnvalue)))) (SplineMesh|GetStartPosition (Utilities|Array|Get(acopy) (Variables|Default|GetSplineMesh) _index))) true)
        (SplineMesh|SetEndPosition (Utilities|Array|Get(acopy) (Variables|Default|GetSplineMesh) _index) (+ (* (* (Math|Vector|GetForwardVector (Variables|Default|GetWindDirection)) (* (Math|Trig|Sin(Radians) (Variables|Default|Gett)) (/ (Variables|Default|GetWindMagnitude) (Variables|Default|GetScale)))) (Math|Trig|Sin(Radians) (Math|Float|MultiplybyPi (/ (Spline|GetDistanceAlongSplineatSplinePoint _spline (+ _index 1)) _returnvalue)))) (SplineMesh|GetEndPosition (Utilities|Array|Get(acopy) (Variables|Default|GetSplineMesh) _index))) true)
        (SplineMesh|SetStartTangent (Utilities|Array|Get(acopy) (Variables|Default|GetSplineMesh) _index) (+ (* (* (Math|Vector|GetForwardVector (Variables|Default|GetWindDirection)) (* (Math|Trig|Cos(Radians) (Variables|Default|Gett)) (* (/ (Variables|Default|GetWindMagnitude) (Variables|Default|GetScale)) 1e+01))) (Math|Trig|Cos(Radians) (Math|Float|MultiplybyPi (/ (Spline|GetDistanceAlongSplineatSplinePoint _spline _index) _returnvalue)))) (SplineMesh|GetStartTangent (Utilities|Array|Get(acopy) (Variables|Default|GetSplineMesh) _index))) true :!class /Script/Engine.SplineMeshComponent)
        (SplineMesh|SetEndTangent (Utilities|Array|Get(acopy) (Variables|Default|GetSplineMesh) _index) (+ (* (* (Math|Vector|GetForwardVector (Variables|Default|GetWindDirection)) (* (Math|Trig|Cos(Radians) (Variables|Default|Gett)) (* (/ (Variables|Default|GetWindMagnitude) (Variables|Default|GetScale)) 1e+01))) (Math|Trig|Cos(Radians) (Math|Float|MultiplybyPi (/ (Spline|GetDistanceAlongSplineatSplinePoint _spline (+ _index 1)) _returnvalue)))) (SplineMesh|GetEndTangent (Utilities|Array|Get(acopy) (Variables|Default|GetSplineMesh) _index))) true :!class /Script/Engine.SplineMeshComponent))))
  (Variables|Default|Sett (+ (Variables|Default|Gett) DeltaSeconds)))

(fn ConstructionScript
  (bind _scale (Variables|Default|GetScale))
  (bind _spline (Variables|Default|GetSpline))
  (Utilities|Array|Clear (Variables|Default|GetSplineMesh))
  (Variables|Default|SetVectorScale (Math|Vector2D|MakeVector2D _scale _scale))
  (for _index (range 0 (- (Spline|GetNumberOfSplinePoints (Variables|Default|GetSpline)) 2))
    (LocalVariables|Setindex _index)
    (Utilities|FlowControl|Sequence
      (:then_0
        (bind _returnvalue (AddComponent|AddSplineMeshComponent true))
        (Utilities|Array|Add (Variables|Default|GetSplineMesh) _returnvalue)
        (Utilities|FlowControl|Sequence
          (:then_0
            (Components|StaticMesh|SetStaticMesh (Utilities|Array|Get(acopy) (Variables|Default|GetSplineMesh) (LocalVariables|Getindex)) (Variables|Default|GetMesh))
            (SplineMesh|SetSplineUpDir (Utilities|Array|Get(acopy) (Variables|Default|GetSplineMesh) (LocalVariables|Getindex)) (Variables|Default|GetSplineUpDirection) true))
          (:then_1
            (Collision|SetCollisionEnabled (Utilities|Array|Get(acopy) (Variables|Default|GetSplineMesh) (LocalVariables|Getindex)) "NoCollision")
            (Rendering|SetCastShadow (Utilities|Array|Get(acopy) (Variables|Default|GetSplineMesh) (LocalVariables|Getindex)) (Variables|Default|GetDynamicShadow))
            (Class|SceneComponent|Attachto (Utilities|Array|Get(acopy) (Variables|Default|GetSplineMesh) (LocalVariables|Getindex)) (Variables|Default|GetDefaultSceneRoot) "None" "KeepRelativeOffset" false))))
      (:then_1
        (SplineMesh|SetStartandEnd (Utilities|Array|Get(acopy) (Variables|Default|GetSplineMesh) (LocalVariables|Getindex)) (.Location (Spline|GetLocationandTangentatSplinePoint _spline (LocalVariables|Getindex) "Local")) (.Tangent (Spline|GetLocationandTangentatSplinePoint _spline (LocalVariables|Getindex) "Local")) (.Location (Spline|GetLocationandTangentatSplinePoint _spline (+ (LocalVariables|Getindex) 1) "Local")) (.Tangent (Spline|GetLocationandTangentatSplinePoint _spline (+ (LocalVariables|Getindex) 1) "Local")) true :!class /Script/Engine.SplineMeshComponent)
        (SplineMesh|SetStartScale (Utilities|Array|Get(acopy) (Variables|Default|GetSplineMesh) (LocalVariables|Getindex)) (Variables|Default|GetVectorScale) true :!class /Script/Engine.SplineMeshComponent)
        (SplineMesh|SetEndScale (Utilities|Array|Get(acopy) (Variables|Default|GetSplineMesh) (LocalVariables|Getindex)) (Variables|Default|GetVectorScale) true :!class /Script/Engine.SplineMeshComponent)))))

(fn GetSplineMesh
  (return (Variables|Default|GetSplineMesh)))