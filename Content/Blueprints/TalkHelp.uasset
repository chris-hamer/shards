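; TalkHelp is an actor that shows a billboard, apparently a talk prompt, when the player is nearby and not in dialogue.
; BeginPlay casts the player pawn to Auyron and caches it, and Tick retries that cast whenever the reference is invalid.
; Each Tick toggles the MaterialBillboard's visibility from its distance to the player and the player's dialogue state.
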(event `self.ReceiveBeginPlay`
  (bind _asauyron (cast `Auyron` (`GameplayStatics.GetPlayerPawn` 0) :!label _label))
  (set `self.Player` _asauyron))

(event `self.ReceiveActorBeginOverlap`
  (params (OtherActor :type "Actor Object Reference")))

(event `self.ReceiveTick`
  (params (DeltaSeconds :type "Float (single-precision)"))
  (bind _materialbillboard (`self.MaterialBillboard`))
  (bind _player (`self.Player`))
  (`/Engine/EditorBlueprintResources/StandardMacros.IsValid` (`self.Player`)
    (:`Is Valid`
      (bind _returnvalue (`Auyron.GetIsInDialogue` _player))
      (if (and (< (`KismetMathLibrary.VSize` (- (`SceneComponent.K2_GetComponentLocation` _materialbillboard) (`self.K2_GetActorLocation` _player))) 1000.0) (not _returnvalue))
        (`SceneComponent.SetVisibility` _materialbillboard true false)
        (else
          (`SceneComponent.SetVisibility` _materialbillboard false false))))
    (:`Is Not Valid`
      (goto _label))))

(fn `UserConstructionScript`)