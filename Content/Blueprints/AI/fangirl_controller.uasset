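; AI controller for the fangirl character that hands its behavior to a behavior tree.
; On BeginPlay it sets up the Testbb blackboard and runs the Fangirl_bt tree.
; Leftover graph nodes for moving toward the player pawn, with a distance check, are disconnected from any event and never execute.
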(event `self.ReceiveBeginPlay`
  (`self.UseBlackboard` "/Game/Blueprints/testbb.testbb")
  (`self.RunBehaviorTree` "/Game/Blueprints/AI/fangirl_bt.fangirl_bt"))

(event `self.ReceiveTick`
  (params (DeltaSeconds :type "Float (single-precision)")))

(fn `UserConstructionScript`)