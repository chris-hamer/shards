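; Fountain trigger actor that reactivates a fan and plays a one-time cutscene when its Activate function is called.
; Activate only sets a flag, which Tick polls through a DoOnce, retrying the Auyron player cast until the reference is valid.
; The sequence activates Fb, whitens the gem, blocks input during a timed Matinee, then restores input and queues a dialogue line.
; Deactivate is empty.
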(event `self.ReceiveBeginPlay`
  (bind _asauyron (cast `Auyron` (`GameplayStatics.GetPlayerPawn` 0) :!label _label))
  (set `self.Player` _asauyron))

(event `self.ReceiveActorBeginOverlap`
  (params (OtherActor :type "Actor Object Reference")))

(event `self.ReceiveTick`
  (params (DeltaSeconds :type "Float (single-precision)"))
  (bind _player (`self.Player`))
  (bind _cut (`self.cut`))
  (bind _fb (`self.fb`))
  (`/Engine/EditorBlueprintResources/StandardMacros.IsValid` (`self.Player`)
    (:`Is Valid`
      (if (`self.DoTheThing`)
        (`/Engine/EditorBlueprintResources/StandardMacros.DoOnce` false
          (:`Completed`
            (if (`KismetSystemLibrary.IsValid` _fb)
              (`/Game/Blueprints/Fan_Blueprint.Activate` _fb)
              (`PrimitiveComponent.SetMaterial` (`StaticMeshActor.StaticMeshComponent` (`self.Gem`)) 0 "/Game/Textures/White.White")
              (`Auyron.BlockInput` _player)
              (`KismetSystemLibrary.Delay` (`self.PreCutscenePause`))
              (`MatineeActor.Play` (`self.Matinee`))
              (`KismetSystemLibrary.Delay` (`self.CutsceneLength`))
              (`Auyron.ResumeInput` _player)
              (`DialogueCut.SetText` _cut "Good job there, kid. If ya don't mind I'm gonna sit back\\nand take in this newly-reactivated-fan aesthetic for a bit.")
              (`DialogueCut.SetNext` _cut null))))))
    (:`Is Not Valid`
      (goto _label))))

(fn `Activate`
  (set `self.DoTheThing` true))

(fn `Deactivate`)

(fn `UserConstructionScript`)