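; Tardis Blueprint that swaps the streamed level behind two closed doors, so the doors reopen onto a different space.
; Activate and Deactivate both trigger the same sequence: close both doors, wait briefly, swap levels, then reopen.
; A looping, non-random MultiGate cycles through three sublevels in order, unloading the previous one and loading the next as visible without blocking.
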(event `CustomEvent_0`
  (`/Game/Blueprints/tardis_door.Close` (`self.door1`) :!label _label)
  (`/Game/Blueprints/tardis_door.Close` (`self.door2`))
  (`KismetSystemLibrary.Delay` 0.5)
  (`|MultiGate` false true
    (:`Out 0`
      (`GameplayStatics.UnloadStreamLevel` "what2")
      (`GameplayStatics.LoadStreamLevel` "what3" true))
    (:`Out 1`
      (`GameplayStatics.UnloadStreamLevel` "what3")
      (`GameplayStatics.LoadStreamLevel` "what4" true))
    (:`Out 2`
      (`GameplayStatics.UnloadStreamLevel` "what4")
      (`GameplayStatics.LoadStreamLevel` "what2" true)))
  (`/Game/Blueprints/tardis_door.Open` (`self.door1`))
  (`/Game/Blueprints/tardis_door.Open` (`self.door2`)))

(event `CustomEvent_1`
  (goto _label))

(fn `Activate`
  (`self.CustomEvent_1`))

(fn `Deactivate`
  (`self.CustomEvent_0`))

(fn `UserConstructionScript`)