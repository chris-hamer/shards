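; Player controller for the Shards character that creates the HUD and handles pausing.
; BeginPlay caches the pawn and sets its mesh to the Anim_Auyron2 animation class.
; Pause and velocity-display inputs use FlipFlops; pausing switches input mode and cursor, then animates and focuses HUD screens.
; Tick writes the controller's location and a zero velocity to the Playerinfo material parameter collection; its dialogue and pause branches are empty.
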(event `InputAction|ToggleVelocityDisplay`
  (params (Key :type "Key Structure" :default "AnyKey"))
  (:`Pressed`
    (`/Engine/EditorBlueprintResources/StandardMacros.FlipFlop`
      (:`A`
        (set `self.DisplayVelocity` true))
      (:`B`
        (set `self.DisplayVelocity` false)))))

(event `InputAction|Pause` :consume false :paused true :overrideparent false
  (params (Key :type "Key Structure" :default "AnyKey"))
  (bind _hud (`self.HUD`))
  (:`Pressed`
    (`/Engine/EditorBlueprintResources/StandardMacros.FlipFlop`
      (:`A`
        (`GameplayStatics.SetGamePaused` true)
        (set `self.bShowMouseCursor` true)
        (`WidgetBlueprintLibrary.SetInputMode_GameAndUIEx` self null false false)
        (`/Game/Blueprints/HUD.AnimateStatsScreen` _hud)
        (`/Game/Blueprints/HUD.AnimateOptionsScreen` _hud)
        (`KismetSystemLibrary.Delay` 0.1)
        (`/Game/Blueprints/HUD.SetFocus` _hud))
      (:`B`
        (`GameplayStatics.SetGamePaused` false)
        (set `self.bShowMouseCursor` false)
        (`WidgetBlueprintLibrary.SetInputMode_GameOnly` self)
        (`ShardsCharacter.HandlePause` (`self.NewVar_0`))))))

(event `self.ReceiveBeginPlay`
  (bind _returnvalue (`|CreateWidget` "/Game/Blueprints/HUD.HUD_C" self))
  (bind _output_get (set `self.HUD` _returnvalue))
  (`UserWidget.AddToViewport` _output_get 0)
  (bind _asshards_character (cast `ShardsCharacter` (`self.K2_GetPawn`)))
  (bind _output_get_2 (set `self.NewVar_0` _asshards_character))
  (bind _returnvalue_2 (`ShardsCharacter.GetMesh` _output_get_2))
  (`SkeletalMeshComponent.SetAnimInstanceClass` _returnvalue_2 "/Game/Generic/Characters/Auyron/Anim_Auyron2.Anim_Auyron2_C"))

(event `self.ReceiveTick`
  (params (DeltaSeconds :type "Float (single-precision)"))
  (bind _newvar_0 (`self.NewVar_0`))
  (`/Engine/EditorBlueprintResources/StandardMacros.IsValid` _newvar_0
    (:`Is Valid`
      (`ShardsCharacter.GetPlayerVelocity` _newvar_0)
      (bind _returnvalue (`ShardsCharacter.GetIsInDialogue` _newvar_0))
      (if _returnvalue
        _
        (else
          _))
      (if (`GameplayStatics.IsGamePaused`)
        _
        (else
          _))
      (`KismetMaterialLibrary.SetVectorParameterValue` "/Game/Meta/playerinfo.playerinfo" "PlayerLocation" (make `LinearColor` (.x (`self.K2_GetActorLocation`)) (.y (`self.K2_GetActorLocation`)) (.z (`self.K2_GetActorLocation`))))
      (`KismetMaterialLibrary.SetVectorParameterValue` "/Game/Meta/playerinfo.playerinfo" "PlayerVelocity" (make `LinearColor` (.x (0.0 0.0 0.0)) (.y (0.0 0.0 0.0)) (.z (0.0 0.0 0.0)))))))

(fn `UserConstructionScript`)