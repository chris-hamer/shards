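; Spline mesh vines Blueprint that gives its vine meshes a leaf material matched to a scale value.
; After the parent construction script runs, it loops over the SplineMesh array, creating a dynamic instance of VineLeaf_Mat per index.
; Each valid mesh gets that instance on material slot 1, with its SplineScale parameter driven by Scale.
; All work happens at construction, as the event graph holds only disabled stubs.
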(fn `UserConstructionScript`
  (bind _splinemesh (`self.SplineMesh`))
  (`parent.UserConstructionScript`)
  (for _index (range (+ (`KismetArrayLibrary.Array_Length` _splinemesh) 1))
    (bind _returnvalue (`KismetMaterialLibrary.CreateDynamicMaterialInstance` "/Game/Generic/Environment/Foliage/VineLeaf_Mat.VineLeaf_Mat"))
    (bind _item (`KismetArrayLibrary.Array_Get` _splinemesh _index))
    (`/Engine/EditorBlueprintResources/StandardMacros.IsValid` _item
      (:`Is Valid`
        (`PrimitiveComponent.SetMaterial` _item 1 _returnvalue)
        (`MaterialInstanceDynamic.SetScalarParameterValue` _returnvalue "SplineScale" (`self.Scale`))))))