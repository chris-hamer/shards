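; Blueprint that feeds the player pawn's world location into the material on its Cube component.
; BeginPlay creates a dynamic material instance from Base, applies it to the Cube and caches player pawn 0.
; Every Tick converts the pawn's location to a linear color and writes it to the "Pos" vector parameter, so the material can react to player position.
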(event `self.ReceiveBeginPlay`
  (`|ExecutionSequence`
    (:`then_0`
      (bind _returnvalue (`KismetMaterialLibrary.CreateDynamicMaterialInstance` (`self.base`)))
      (bind _output_get (set `self.mat` _returnvalue))
      (`PrimitiveComponent.SetMaterial` (`self.Cube`) 0 _output_get))
    (:`then_1`
      (set `self.player` (`GameplayStatics.GetPlayerPawn` 0)))))

(event `self.ReceiveTick`
  (params (DeltaSeconds :type "Float (single-precision)"))
  (`MaterialInstanceDynamic.SetVectorParameterValue` (`self.mat`) "Pos" (`KismetMathLibrary.Conv_VectorToLinearColor` (`self.K2_GetActorLocation` (`self.player`)))))

(fn `UserConstructionScript`)