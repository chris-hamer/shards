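; Player controller that creates the HUD widget at BeginPlay and handles pausing for the player's Auyron pawn.
; The Pause input flip-flops between pausing with a visible cursor and Game and UI input focused on the HUD, and resuming with game-only input.
; BeginPlay also caches the controlled Auyron, whose dialogue state Tick checks alongside the pause state without acting on either.
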(event `InputAction|Pause` :consume false :paused true :overrideparent false
  (params (Key :type "Key Structure" :default "AnyKey"))
  (:`Pressed`
    (`/Engine/EditorBlueprintResources/StandardMacros.FlipFlop`
      (:`A`
        (`GameplayStatics.SetGamePaused` true)
        (set `self.bShowMouseCursor` true)
        (`WidgetBlueprintLibrary.SetInputMode_GameAndUIEx` self (`self.NewVar_1`) false false))
      (:`B`
        (`GameplayStatics.SetGamePaused` false)
        (set `self.bShowMouseCursor` false)
        (`WidgetBlueprintLibrary.SetInputMode_GameOnly` self)))))

(event `self.ReceiveBeginPlay`
  (bind _returnvalue (`|CreateWidget` "/Game/HUD.HUD_C" self))
  (bind _output_get (set `self.NewVar_1` _returnvalue))
  (`UserWidget.AddToViewport` _output_get 0)
  (bind _asauyron (cast `Auyron` (`self.K2_GetPawn`)))
  (set `self.NewVar_0` _asauyron))

(event `self.ReceiveTick`
  (params (DeltaSeconds :type "Float (single-precision)"))
  (bind _returnvalue (`Auyron.GetIsInDialogue` (`self.NewVar_0`)))
  (if _returnvalue
    (if (`GameplayStatics.IsGamePaused`)
      _)))

(fn `UserConstructionScript`)