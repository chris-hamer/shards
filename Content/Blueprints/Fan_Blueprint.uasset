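; Fan actor that pushes with a force region while showing a "Woosh" particle effect and a spinning blade, switched on or off at start by StartEnabled.
; Activate and Deactivate toggle the particle emitter, the force region and the blade component together.
; Each call also propagates to an optional linked Next reference, so a chain of fans switches as one.
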(event `self.ReceiveBeginPlay`
  (`ParticleSystemComponent.SetEmitterEnable` (`Emitter.ParticleSystemComponent` (`self.particles`)) "Woosh" true)
  (if (`self.StartEnabled`)
    (`self.Activate`)
    (else
      (`self.Deactivate`))))

(event `self.ReceiveActorBeginOverlap`
  (params (OtherActor :type "Actor Object Reference")))

(event `self.ReceiveTick`
  (params (DeltaSeconds :type "Float (single-precision)")))

(fn `Activate`
  (bind _next (`self.Next`))
  (`ParticleSystemComponent.SetEmitterEnable` (`Emitter.ParticleSystemComponent` (`self.particles`)) "Woosh" true)
  (`ForceRegion.Enable` (`self.force region`))
  (`MovingPlatform.Activate` (`self.fan blade`))
  (if (`KismetSystemLibrary.IsValid` _next)
    (`self.Activate` _next)))

(fn `Deactivate`
  (bind _next (`self.Next`))
  (`ParticleSystemComponent.SetEmitterEnable` (`Emitter.ParticleSystemComponent` (`self.particles`)) "Woosh" false)
  (`ForceRegion.Disable` (`self.force region`))
  (`MovingPlatform.Deactivate` (`self.fan blade`))
  (if (`KismetSystemLibrary.IsValid` _next)
    (`self.Deactivate` _next)))

(fn `UserConstructionScript`)