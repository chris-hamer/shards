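; Game mode that smoothly blends the level's cel-shading look, lighting and music toward target values stored in its variables.
; BeginPlay seeds light range and tint targets from the CelShaderInfo parameter collection, then Tick interpolates the collection toward them.
; The interpolated UseTint value also inversely drives DayNight's light scale and scales indoor light intensities from their default brightness.
; Tick crossfades music whenever the current track changes.
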(event `self.ReceiveBeginPlay`
  (bind _returnvalue (`KismetMaterialLibrary.GetScalarParameterValue` "/Game/Textures/CelShaderInfo.CelShaderInfo" "LightMin"))
  (set `self.LightMin` _returnvalue)
  (bind _returnvalue_2 (`KismetMaterialLibrary.GetScalarParameterValue` "/Game/Textures/CelShaderInfo.CelShaderInfo" "LightMax"))
  (set `self.LightMax` _returnvalue_2)
  (bind _returnvalue_3 (`KismetMaterialLibrary.GetVectorParameterValue` "/Game/Textures/CelShaderInfo.CelShaderInfo" "TintColor"))
  (set `self.Tint` _returnvalue_3))

(event `self.ReceiveTick`
  (params (DeltaSeconds :type "Float (single-precision)"))
  (bind _prevmusic (`self.prevmusic`))
  (bind _currentmusic (`self.currentmusic`))
  (`|ExecutionSequence`
    (:`then_0`
      (bind _returnvalue (`KismetMaterialLibrary.GetScalarParameterValue` "/Game/Textures/CelShaderInfo.CelShaderInfo" "LightMin"))
      (`KismetMaterialLibrary.SetScalarParameterValue` "/Game/Textures/CelShaderInfo.CelShaderInfo" "LightMin" (`KismetMathLibrary.FInterpTo` _returnvalue (`self.LightMin`) DeltaSeconds 1.0)))
    (:`then_1`
      (bind _returnvalue_2 (`KismetMaterialLibrary.GetScalarParameterValue` "/Game/Textures/CelShaderInfo.CelShaderInfo" "LightMax"))
      (`KismetMaterialLibrary.SetScalarParameterValue` "/Game/Textures/CelShaderInfo.CelShaderInfo" "LightMax" (`KismetMathLibrary.FInterpTo` _returnvalue_2 (`self.LightMax`) DeltaSeconds 1.0)))
    (:`then_2`
      (bind _returnvalue_3 (`KismetMaterialLibrary.GetScalarParameterValue` "/Game/Textures/CelShaderInfo.CelShaderInfo" "UseTint"))
      (bind _returnvalue_4 (`KismetMathLibrary.FInterpTo` _returnvalue_3 (`self.TargetValue`) DeltaSeconds 1.0))
      (`KismetMaterialLibrary.SetScalarParameterValue` "/Game/Textures/CelShaderInfo.CelShaderInfo" "UseTint" _returnvalue_4)
      (set `/Game/Blueprints/daynight.LightScale` (- 1.0 _returnvalue_4) (`self.DayNight`))
      (for (_array_element _array_index) (`self.IndoorLights`)
        (`/Engine/EditorBlueprintResources/StandardMacros.IsValid` _array_element
          (:`Is Valid`
            (`LightComponent.SetIntensity` (`Light.LightComponent` _array_element) (* (`KismetArrayLibrary.Array_Get` (`self.DefaultBrightness`) _array_index) _returnvalue_4))))))
    (:`then_3`
      (bind _returnvalue_5 (`KismetMaterialLibrary.GetVectorParameterValue` "/Game/Textures/CelShaderInfo.CelShaderInfo" "TintColor"))
      (`KismetMaterialLibrary.SetVectorParameterValue` "/Game/Textures/CelShaderInfo.CelShaderInfo" "TintColor" (`KismetMathLibrary.CInterpTo` _returnvalue_5 (`self.Tint`) DeltaSeconds 1.0)))
    (:`then_4`
      (if (!= (`self.currentmusic`) (`self.prevmusic`))
        (`/Engine/EditorBlueprintResources/StandardMacros.IsValid` _prevmusic
          (:`Is Valid`
            (`AudioComponent.FadeOut` _prevmusic 1.0 0.0))
          (:`Is Not Valid`
            _))
        (`/Engine/EditorBlueprintResources/StandardMacros.IsValid` _currentmusic
          (:`Is Valid`
            (`AudioComponent.FadeIn` _currentmusic 1.0 1.0 0.0))
          (:`Is Not Valid`
            _))
        (set `self.prevmusic` (`self.currentmusic`))))
    (:`then_5`
      (bind _returnvalue_6 (`KismetMaterialLibrary.GetScalarParameterValue` "/Game/Textures/CelShaderInfo.CelShaderInfo" "LightMin")))))

(fn `UserConstructionScript`)