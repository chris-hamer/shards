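; island_switch is a switch Blueprint that, once activated, plays a one-time cutscene.
; Activate turns on its light and sets an Isactive flag, which Tick polls behind a DoOnce.
; The sequence blocks player input, pauses briefly, plays the cutscene, waits for its length, then restores input.
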(event `self.ReceiveBeginPlay`)

(event `self.ReceiveActorBeginOverlap`
  (params (OtherActor :type "Actor Object Reference")))

(event `self.ReceiveTick`
  (params (DeltaSeconds :type "Float (single-precision)"))
  (bind _player (`self.Player`))
  (if (`self.isactive`)
    (`/Engine/EditorBlueprintResources/StandardMacros.DoOnce` false
      (:`Completed`
        (`Auyron.BlockInput` _player)
        (`KismetSystemLibrary.Delay` (`self.PrecutscenePauseDuration`))
        (`MatineeActor.Play` (`self.Cutscene`))
        (`KismetSystemLibrary.Delay` (`self.CutsceneLength`))
        (`Auyron.ResumeInput` _player)))))

(fn `Activate`
  (`SceneComponent.SetVisibility` (`Light.LightComponent` (`self.light`)) true false)
  (set `self.isactive` true))

(fn `UserConstructionScript`)