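; Day-night cycle actor that continuously rolls a directional light through a full turn over DayLength.
; Each tick it writes the normalized roll to TimeOfDay in the Worldinfo material parameter collection.
; The same roll drives power curves that fade the sun out and moonlight in, scaled by the sun's starting intensity, with moonlight keeping a small minimum.
; It also prints the moonlight factor every frame for debugging.
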(event `self.ReceiveBeginPlay`
  (set `self.startrot` (`SceneComponent.K2_GetComponentRotation` (`self.DirectionalLight`)))
  (set `self.MaxBrightness` (`LightComponentBase.Intensity` (`self.DirectionalLight`))))

(event `self.ReceiveTick`
  (params (DeltaSeconds :type "Float (single-precision)"))
  (bind _directionallight (`self.DirectionalLight`))
  (bind _returnvalue (/ (`KismetMathLibrary.DegreesToRadians` (.roll (`SceneComponent.K2_GetComponentRotation` _directionallight))) (`KismetMathLibrary.MultiplyByPi` 1.0)))
  (bind _returnvalue_2 (`KismetMathLibrary.FClamp` (* (`KismetMathLibrary.Abs` _returnvalue) 2.0)))
  (bind _returnvalue_3 (`KismetMathLibrary.FClamp` (- (`KismetMathLibrary.MultiplyMultiply_FloatFloat` _returnvalue_2 32.0) -0.1)))
  (`SceneComponent.K2_AddWorldRotation` _directionallight (`KismetMathLibrary.MakeRotator` (* DeltaSeconds (/ 360.0 (`self.DayLength`)))) false false)
  (`KismetMaterialLibrary.SetScalarParameterValue` "/Game/wbp/worldinfo.worldinfo" "TimeOfDay" _returnvalue)
  (`LightComponent.SetIntensity` (`self.DirectionalLight`) (* (`KismetMathLibrary.MultiplyMultiply_FloatFloat` (- 1.0 _returnvalue_2) 0.125) (`self.MaxBrightness`)))
  (`LightComponent.SetIntensity` (`self.Moonlight`) (* _returnvalue_3 (`self.MaxBrightness`)))
  (`KismetSystemLibrary.PrintString` (`KismetStringLibrary.Conv_DoubleToString` _returnvalue_3)))

(fn `UserConstructionScript`)