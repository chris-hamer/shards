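; TARDIS door actor that slides between an open and a closed position.
; Open and Close events set the target location to the stored Start and End vectors respectively.
; Tick continuously lerps the actor toward that target by a delta-time-scaled alpha, giving a quick ease-out move without a timeline or sweep.
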(event `self.ReceiveBeginPlay`)

(event `self.ReceiveActorBeginOverlap`
  (params (OtherActor :type "Actor Object Reference")))

(event `self.ReceiveTick`
  (params (DeltaSeconds :type "Float (single-precision)"))
  (`self.K2_SetActorLocation` (`KismetMathLibrary.VLerp` (`self.K2_GetActorLocation`) (`self.Dest`) (* DeltaSeconds 16.0))))

(event `Open`
  (set `self.Dest` (`self.Start`)))

(event `Close`
  (set `self.Dest` (`self.End`)))

(fn `UserConstructionScript`)