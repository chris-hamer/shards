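; Blueprint that drops a referenced Wings actor along its local Z axis with increasing speed.
; Each Tick offsets Wings by a stored vector, unscaled by frame time, with sweep and teleport enabled.
; While that vector's Z is above -900, it unhides Wings and grows the downward step using delta time.
; Switch checks are disconnected, and Activate is empty.
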(event `self.ReceiveBeginPlay`)

(event `self.ReceiveActorBeginOverlap`
  (params (OtherActor :type "Actor Object Reference")))

(event `self.ReceiveTick`
  (params (DeltaSeconds :type "Float (single-precision)"))
  (bind _wings (`self.wings`))
  (`self.K2_AddActorLocalOffset` _wings (stale _output_get) true true)
  (if (and (> (.z (`self.asdfasdf`)) -900.0) true true)
    (`self.SetActorHiddenInGame` _wings false)
    (bind _output_get (set `self.asdfasdf` (+ (* (`KismetMathLibrary.MakeVector` 0.0 0.0 -100.0) DeltaSeconds) (`self.asdfasdf`))))))

(fn `Activate`)

(fn `UserConstructionScript`)