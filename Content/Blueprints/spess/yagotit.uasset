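; Blueprint that triggers a one-time cutscene once its referenced Pickup is no longer valid, presumably after the player takes it.
; Tick polls the Pickup reference and uses a DoOnce so the sequence runs only once.
; The sequence blocks player input, waits a configurable pause, plays the Cutscene, waits out its length, then restores input.
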(event `self.ReceiveTick`
  (params (DeltaSeconds :type "Float (single-precision)"))
  (bind _player (`self.Player`))
  (`/Engine/EditorBlueprintResources/StandardMacros.IsValid` (`self.Pickup`)
    (:`Is Not Valid`
      (`/Engine/EditorBlueprintResources/StandardMacros.DoOnce` false
        (:`Completed`
          (`Auyron.BlockInput` _player)
          (`KismetSystemLibrary.Delay` (`self.PrecutscenePauseDuration`))
          (`MatineeActor.Play` (`self.Cutscene`))
          (`KismetSystemLibrary.Delay` (`self.CutsceneLength`))
          (`Auyron.ResumeInput` _player))))))

(fn `UserConstructionScript`)