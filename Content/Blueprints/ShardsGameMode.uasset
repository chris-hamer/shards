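; Game mode for Shards that smoothly blends cel-shading and lighting toward target values held in its variables.
; BeginPlay seeds light range and tint targets from the CelShaderInfo parameter collection, and Tick interpolates the collection toward them.
; The UseTint blend also inversely drives DayNight's light scale and scales indoor lights from their default brightness, when DayNight is valid.
; Music-switching and debug print nodes are disconnected.
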(event `self.ReceiveBeginPlay`
  (bind _returnvalue (`KismetMaterialLibrary.GetScalarParameterValue` "/Game/Meta/CelShaderInfo.CelShaderInfo" "LightMin"))
  (set `self.LightMin` _returnvalue)
  (bind _returnvalue_2 (`KismetMaterialLibrary.GetScalarParameterValue` "/Game/Meta/CelShaderInfo.CelShaderInfo" "LightMax"))
  (set `self.LightMax` _returnvalue_2)
  (bind _returnvalue_3 (`KismetMaterialLibrary.GetVectorParameterValue` "/Game/Meta/CelShaderInfo.CelShaderInfo" "TintColor"))
  (set `self.Tint` _returnvalue_3))

(event `self.ReceiveTick`
  (params (DeltaSeconds :type "Float (single-precision)"))
  (bind _daynight (`self.DayNight`))
  (`|ExecutionSequence`
    (:`then_0`
      (bind _returnvalue (`KismetMaterialLibrary.GetScalarParameterValue` "/Game/Meta/CelShaderInfo.CelShaderInfo" "LightMin"))
      (`KismetMaterialLibrary.SetScalarParameterValue` "/Game/Meta/CelShaderInfo.CelShaderInfo" "LightMin" (`KismetMathLibrary.FInterpTo` _returnvalue (`self.LightMin`) DeltaSeconds 1.0)))
    (:`then_1`
      (bind _returnvalue_2 (`KismetMaterialLibrary.GetScalarParameterValue` "/Game/Meta/CelShaderInfo.CelShaderInfo" "LightMax"))
      (`KismetMaterialLibrary.SetScalarParameterValue` "/Game/Meta/CelShaderInfo.CelShaderInfo" "LightMax" (`KismetMathLibrary.FInterpTo` _returnvalue_2 (`self.LightMax`) DeltaSeconds 1.0)))
    (:`then_2`
      (bind _returnvalue_3 (`KismetMaterialLibrary.GetScalarParameterValue` "/Game/Meta/CelShaderInfo.CelShaderInfo" "UseTint"))
      (bind _returnvalue_4 (`KismetMathLibrary.FInterpTo` _returnvalue_3 (`self.TargetValue`) DeltaSeconds 1.0))
      (`KismetMaterialLibrary.SetScalarParameterValue` "/Game/Meta/CelShaderInfo.CelShaderInfo" "UseTint" _returnvalue_4)
      (`/Engine/EditorBlueprintResources/StandardMacros.IsValid` _daynight
        (:`Is Valid`
          (set `/Game/Effects/DayNight/daynight.LightScale` (- 1.0 _returnvalue_4) _daynight)
          (for (_array_element _array_index) (`self.IndoorLights`)
            (`/Engine/EditorBlueprintResources/StandardMacros.IsValid` _array_element
              (:`Is Valid`
                (`LightComponent.SetIntensity` (`Light.LightComponent` _array_element) (* (`KismetArrayLibrary.Array_Get` (`self.DefaultBrightness`) _array_index) _returnvalue_4))))))))
    (:`then_3`
      (bind _returnvalue_5 (`KismetMaterialLibrary.GetVectorParameterValue` "/Game/Meta/CelShaderInfo.CelShaderInfo" "TintColor"))
      (`KismetMaterialLibrary.SetVectorParameterValue` "/Game/Meta/CelShaderInfo.CelShaderInfo" "TintColor" (`KismetMathLibrary.CInterpTo` _returnvalue_5 (`self.Tint`) DeltaSeconds 1.0)))
    (:`then_5`
      (bind _returnvalue_6 (`KismetMaterialLibrary.GetScalarParameterValue` "/Game/Meta/CelShaderInfo.CelShaderInfo" "LightMin")))))

(fn `UserConstructionScript`)