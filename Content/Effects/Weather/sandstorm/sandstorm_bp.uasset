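; Sandstorm weather effect actor that follows the player's Auyron pawn.
; Each tick it moves itself to a large fixed Y offset from the player with a constant rotation, then places its particle system at the player's location.
; The player reference is cached on BeginPlay, and Tick retries the cast whenever that reference is invalid.
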(event `self.ReceiveBeginPlay`
  (bind _asauyron (cast `Auyron` (`GameplayStatics.GetPlayerPawn` 0) :!label _label))
  (set `self.Player` _asauyron))

(event `self.ReceiveTick`
  (params (DeltaSeconds :type "Float (single-precision)"))
  (bind _player (`self.Player`))
  (bind _returnvalue (`self.K2_GetActorLocation` _player))
  (`/Engine/EditorBlueprintResources/StandardMacros.IsValid` _player
    (:`Is Valid`
      (`self.K2_SetActorLocationAndRotation` (+ _returnvalue (0.0 50000.0 0.0)) (struct :`Yaw` -90.0))
      (`SceneComponent.K2_SetWorldLocationAndRotation` :`self` (`self.ParticleSystem`) :`NewLocation` _returnvalue))
    (:`Is Not Valid`
      (goto _label))))

(fn `UserConstructionScript`)